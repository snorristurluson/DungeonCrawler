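; Character Blueprint that previews a navigation path from itself to the point under the mouse cursor.
; Every Tick, a Sphere component snaps to the impact point of a Visibility trace under the cursor.
; While Left Shift is held, it runs a synchronous navmesh path query to that point and passes the waypoints to PathVisualizer, without moving the character.
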(event EventBeginPlay)

(event Collision|EventActorBeginOverlap
  (params (OtherActor :type Actor%20Object%20Reference)))

(event EventTick
  (params (DeltaSeconds :type Float%20%28single-precision%29))
  (bind _returnvalue (Game|GetPlayerController 0))
  (bind _hitresult (Game|Player|GetHitResultUnderCursorbyChannel _returnvalue "TraceTypeQuery1" true))
  (Transformation|SetWorldLocation (Variables|Default|GetSphere) (.impactpoint _hitresult) false false)
  (if (Game|Player|IsInputKeyDown (Game|GetPlayerController 0) "LeftShift")
    (bind _returnvalue_2 (Class|NavigationSystemV1|FindPathtoLocationSynchronously (Class|NavigationSystemV1|GetNavigationSystem) (Transformation|GetActorLocation) (.impactpoint _hitresult) self 0))
    (Class|PathVisualizerComponent|SetWaypoints (Variables|Default|GetPathVisualizer) (Variables|/Script/NavigationSystem.NavigationPath|GetPathPoints _returnvalue_2))))

(fn ConstructionScript)